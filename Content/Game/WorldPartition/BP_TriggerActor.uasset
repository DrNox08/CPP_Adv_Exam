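; Trigger actor that loads the next room in one of three directions (forward, left, right) as the level is explored.
; Each trigger's overlap checks its matching position marker with a small zero-length sphere trace for blocking objects.
; If the spot is clear, it asks LevelManagementSubsystem to load a room at that marker's location and rotation, then disables that trigger's collision.
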(event OnComponentBeginOverlap(TriggerForward)
  (params (OverlappedComponent :type Primitive%20Component%20Object%20Reference) (OtherActor :type Actor%20Object%20Reference) (OtherComp :type Primitive%20Component%20Object%20Reference) (OtherBodyIndex :type Integer) (bFromSweep :type Boolean) (SweepResult :type Hit%20Result%20Structure%20%28by%20ref%29))
  (bind _forward_position (Variables|Default|GetForward%20Position))
  (bind _returnvalue (Transformation|GetWorldTransform _forward_position))
  (bind _valuie (CallFunction|IsPositionAvailable (.location _returnvalue) (.location _returnvalue)))
  (if _valuie
    (Class|LevelManagementSubsystem|LoadNextRoom (Subsystems|GetLevelManagementSubsystem) (Math|Transform|MakeTransform (.location _returnvalue) (.rotation _returnvalue) "1.000000,1.000000,1.000000") "" 0 false)
    (Collision|SetCollisionEnabled (Variables|Default|GetTrigger%20Forward) "NoCollision")))

(event OnComponentBeginOverlap(TriggerLeft)
  (params (OverlappedComponent :type Primitive%20Component%20Object%20Reference) (OtherActor :type Actor%20Object%20Reference) (OtherComp :type Primitive%20Component%20Object%20Reference) (OtherBodyIndex :type Integer) (bFromSweep :type Boolean) (SweepResult :type Hit%20Result%20Structure%20%28by%20ref%29))
  (bind _left_position (Variables|Default|GetLeft%20Position))
  (bind _returnvalue (Transformation|GetWorldTransform _left_position))
  (bind _valuie (CallFunction|IsPositionAvailable (.location _returnvalue) (.location _returnvalue)))
  (if _valuie
    (Class|LevelManagementSubsystem|LoadNextRoom (Subsystems|GetLevelManagementSubsystem) (Math|Transform|MakeTransform (.location _returnvalue) (.rotation _returnvalue) "1.000000,1.000000,1.000000") "" 0 false)
    (Collision|SetCollisionEnabled (Variables|Default|GetTrigger%20Left) "NoCollision")))

(event OnComponentBeginOverlap(TriggerRight)
  (params (OverlappedComponent :type Primitive%20Component%20Object%20Reference) (OtherActor :type Actor%20Object%20Reference) (OtherComp :type Primitive%20Component%20Object%20Reference) (OtherBodyIndex :type Integer) (bFromSweep :type Boolean) (SweepResult :type Hit%20Result%20Structure%20%28by%20ref%29))
  (bind _right_position (Variables|Default|GetRight%20Position))
  (bind _returnvalue (Transformation|GetWorldTransform _right_position))
  (bind _valuie (CallFunction|IsPositionAvailable (.location _returnvalue) (.location _returnvalue)))
  (if _valuie
    (Class|LevelManagementSubsystem|LoadNextRoom (Subsystems|GetLevelManagementSubsystem) (Math|Transform|MakeTransform (.location _returnvalue) (.rotation _returnvalue) "1.000000,1.000000,1.000000") "" 0 false)
    (Collision|SetCollisionEnabled (Variables|Default|GetTrigger%20Right) "NoCollision")))

(event EventBeginPlay)

(fn ConstructionScript)

(fn IsPositionAvailable
  (params (Start :type Vector) (End :type Vector))
  (bind _returnvalue (Collision|MultiSphereTraceForObjects Start End 2e+01 (Utilities|Array|MakeArray "ObjectTypeQuery1" "ObjectTypeQuery2" "ObjectTypeQuery7") false 0 "None" false))
  (return (not _returnvalue)))