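; BP_MyVoxelActor is a voxel actor that requests pathfinding from the player to a trigger actor's forward point when play begins.
; It takes the target from TriggerForward, requests an asynchronous region around its Origin, waits briefly, then requests the path update.
; A debug sphere marks the player's start position, and a failed path prints a message.
; Other debug drawing nodes are left unconnected.
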(event EventBeginPlay
  (bind _trigger_actor (Variables|Default|GetTrigger%20Actor))
  (bind _trigger_forward (Variables|/Game/Game/WorldPartition/BP_TriggerActor.BP_TriggerActor_C|GetTrigger%20Forward _trigger_actor))
  (bind _returnvalue (Transformation|GetWorldLocation _trigger_forward))
  (Rendering|Debug|DrawDebugSphere (Transformation|GetActorLocation (Game|GetPlayerCharacter 0)) 1e+02 12 "(R=1.000000,G=0.000000,B=0.024246,A=1.000000)" 5.0 3.0)
  (Variables|Default|SetTarget%20Location (Math|Vector|MakeVector (.x _returnvalue) (.y _returnvalue) (.z _returnvalue)))
  (Class|VoxelActor|RequestRegionAsyn (Transformation|GetWorldLocation (Variables|Default|GetOrigin)) 7e+03)
  (Utilities|FlowControl|Delay 0.5)
  (|RequestPathfindingUpdate (Transformation|GetActorLocation (Game|GetPlayerCharacter 0)) (Variables|Default|GetTarget%20Location)
    (:OnFailed
      (Development|PrintString "PATH NOT FOUND"))))

(fn ConstructionScript)