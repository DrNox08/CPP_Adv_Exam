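; BP_VoxelActor appears to be a test actor for a voxel grid and pathfinding system.
; On BeginPlay it requests an async region around itself after a short delay, later drawing debug spheres at its location and a point ahead.
; In parallel, it runs an AsyncDelayWithTick action that prints on each tick and on completion.
; Path requests, including one that draws returned path points, are present but unconnected.
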(event EventBeginPlay
  (bind _self self)
  (bind _rootcomponent (Variables|/Script/Engine.Actor|GetRootComponent _self))
  (bind _returnvalue (Transformation|GetWorldLocation _rootcomponent))
  (Utilities|FlowControl|Sequence
    (:then_0
      (Utilities|FlowControl|Delay 1.0)
      (Class|VoxelActor|RequestRegionAsyn _returnvalue 1e+03)
      (Utilities|FlowControl|Delay 3.0)
      (Rendering|Debug|DrawDebugSphere _returnvalue 1e+02 12 "(R=1.000000,G=0.209844,B=0.007382,A=1.000000)" 1e+01 5.0)
      (Rendering|Debug|DrawDebugSphere (+ _returnvalue (* (Transformation|GetActorForwardVector _self) 5e+02)) 1e+02 12 "(R=0.000000,G=1.000000,B=0.023465,A=1.000000)" 1e+01 5.0))
    (:then_1
      (bind _secondsremaining (|AsyncDelaywithTick 30)
        (:OnTick
          (Development|PrintString (Utilities|String|ToString(Integer) _secondsremaining)))
        (:OnCompleted
          (Development|PrintString "complete"))))))

(event Collision|EventActorBeginOverlap
  (params (OtherActor :type Actor%20Object%20Reference)))

(event EventTick
  (params (DeltaSeconds :type Float%20%28single-precision%29)))

(fn ConstructionScript)